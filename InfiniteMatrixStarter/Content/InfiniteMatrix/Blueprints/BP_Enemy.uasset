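; BP_Enemy is an enemy actor that damages the player on contact and awards score when shot.
; Its Sphere overlap handles two cases: touching BP_Player calls ProcessHit, destroys the enemy, plays a camera shake at the player and displays restart if the player is dead.
; Touching a BP_Projectile adds score to player 0's BP_Player and destroys both the enemy and the projectile.
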(event `self.ReceiveBeginPlay`)

(event `self.Sphere.OnComponentBeginOverlap`
  (params (OverlappedComponent :type "PrimitiveComponent Object Reference") (OtherActor :type "Actor Object Reference") (OtherComp :type "PrimitiveComponent Object Reference") (OtherBodyIndex :type Integer) (bFromSweep :type Boolean) (SweepResult :type "HitResult Structure (by ref)"))
  (`|ExecutionSequence`
    (:`then_0`
      (bind _asbp_player (cast `/Game/InfiniteMatrix/Blueprints/BP_Player` OtherActor))
      (bind _returnvalue (`/Game/InfiniteMatrix/Blueprints/BP_Player.ProcessHit` _asbp_player))
      (`self.K2_DestroyActor`)
      (bind _output_get (set `/Game/InfiniteMatrix/Blueprints/BP_Player.isDead` _returnvalue _asbp_player))
      (`|ExecutionSequence`
        (:`then_0`
          (`GameplayStatics.PlayWorldCameraShake` "/Game/InfiniteMatrix/Blueprints/BP_CameraShake.BP_CameraShake_C" (`self.K2_GetActorLocation` (`GameplayStatics.GetPlayerPawn` 0)) 0.0 500.0))
        (:`then_1`
          (if _output_get
            (`/Game/InfiniteMatrix/Blueprints/BP_Player.DisplayRestart` _asbp_player)))))
    (:`then_1`
      (bind _asbp_projectile (cast `/Game/InfiniteMatrix/Blueprints/BP_Projectile` OtherActor))
      (bind _asbp_player_2 (cast `/Game/InfiniteMatrix/Blueprints/BP_Player` (`GameplayStatics.GetPlayerPawn` 0)))
      (`/Game/InfiniteMatrix/Blueprints/BP_Player.AddScore` _asbp_player_2 50)
      (`self.K2_DestroyActor`)
      (`self.K2_DestroyActor` _asbp_projectile))))

(fn `UserConstructionScript`)